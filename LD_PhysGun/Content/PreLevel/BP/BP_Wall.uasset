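; BP_Wall is a wall actor that lowers out of the way when deactivated.
; It stores its start location on BeginPlay, and DeactivateWall plays the TL_Sink timeline to lerp the actor straight down by SinkDistance without sweeping.
; When the timeline finishes, the Wall component loses collision and is hidden in game.
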(event Custom|DeactivateWall
  (bind _startlocation (Variables|Default|GetStartLocation))
  (bind _alpha (Timeline|TL_Sink PlayFromStart)
    (:Update
      (Transformation|SetActorLocation (Math|Vector|Lerp(Vector) (Variables|Default|GetStartLocation) (Math|Vector|MakeVector (.x _startlocation) (.y _startlocation) (- (.z _startlocation) (Variables|Default|GetSinkDistance))) _alpha) false false))
    (:Finished
      (Collision|SetCollisionEnabled (Variables|Default|GetWall) "NoCollision")
      (Development|SetHiddeninGame (Variables|Default|GetWall) true false))))

(event EventBeginPlay
  (Variables|Default|SetStartLocation (Transformation|GetActorLocation)))

(event Collision|EventActorBeginOverlap
  (params (OtherActor :type Actor%20Object%20Reference)))

(event EventTick
  (params (DeltaSeconds :type Float%20%28single-precision%29)))

(fn ConstructionScript)