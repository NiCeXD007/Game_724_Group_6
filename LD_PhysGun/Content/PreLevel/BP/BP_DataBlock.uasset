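; BP_DataBlock is a physics block that can be absorbed into a target point and replaces itself when moved.
; Shortly after BeginPlay it enables physics and flags itself absorbable.
; Tick watches for displacement from the original location, then once spawns a DataBlockClass copy there after a delay.
; StartAbsorb disables physics and collision, so Tick interpolates location and scale toward the target and destroys the actor on arrival.
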(event Custom|StartAbsorb
  (params (TargetLcation :type Vector))
  (bind _blockmesh (Variables|Default|GetBlockMesh))
  (if (not (Variables|Default|GetbIsAbsorbing))
    (Variables|Default|SetbIsAbsorbing true)
    (Variables|Default|SetAbsorbTargetLocation TargetLcation)
    (Physics|SetSimulatePhysics _blockmesh false)
    (Physics|SetEnableGravity _blockmesh false)
    (Collision|SetCollisionEnabled _blockmesh "NoCollision")))

(event Custom|StartRespawnDelay
  (Utilities|FlowControl|Delay 3.0)
  (Game|SpawnActorfromClass (Variables|Default|GetDataBlockClass) (Math|Transform|MakeTransform (Variables|Default|GetOriginalLocation) "0.000000,0.000000,0.000000" (Variables|Default|GetStartScale)) "Undefined" "MultiplyWithRoot" 0 2e+01 0))

(event EventBeginPlay
  (bind _blockmesh (Variables|Default|GetBlockMesh))
  (Variables|Default|SetStartScale (Transformation|GetActorScale3D))
  (Variables|Default|SetOriginalLocation (Transformation|GetActorLocation))
  (Utilities|FlowControl|Delay 0.2)
  (Variables|Default|SetbCanBeAbsorbed true)
  (Variables|Default|SetbIsAbsorbing false)
  (Variables|Default|SetbHasSpawnReplacement false)
  (Physics|SetSimulatePhysics _blockmesh true)
  (Physics|SetEnableGravity _blockmesh true)
  (Collision|SetCollisionEnabled _blockmesh "QueryAndPhysics"))

(event Collision|EventActorBeginOverlap
  (params (OtherActor :type Actor%20Object%20Reference)))

(event EventTick
  (params (DeltaSeconds :type Float%20%28single-precision%29))
  (Utilities|FlowControl|Sequence
    (:then_0
      ;[0.15 0.15 0.15 0.5] Spawn
      (if (and (> (Math|Vector|Distance(Vector) (Transformation|GetActorLocation) (Variables|Default|GetOriginalLocation)) 1e+02) (not (Variables|Default|GetbHasSpawnReplacement)))
        (Variables|Default|SetbHasSpawnReplacement true)
        (CallFunction|StartRespawnDelay)))
    (:then_1
      (if (Variables|Default|GetbIsAbsorbing)
        ;[0.15 0.15 0.15 0.5] Location Difference
        (Transformation|SetActorLocation (Math|Interpolation|VInterpTo (Transformation|GetActorLocation) (Variables|Default|GetAbsorbTargetLocation) DeltaSeconds (Variables|Default|GetAbsorbSpeed)) false false)
        ;[0.15 0.15 0.15 0.5] ScaleDifference
        (Transformation|SetActorScale3D (Math|Interpolation|VInterpTo (Transformation|GetActorScale3D) "0.500000,0.500000,0.500000" DeltaSeconds (Variables|Default|GetAbsorbSpeed)))
        ;[0.15 0.15 0.15 0.5] Absorbed
        (if (<= (Math|Vector|Distance(Vector) (Transformation|GetActorLocation) (Variables|Default|GetAbsorbTargetLocation)) 15.0)
          (Actor|DestroyActor))))))

(fn ConstructionScript)