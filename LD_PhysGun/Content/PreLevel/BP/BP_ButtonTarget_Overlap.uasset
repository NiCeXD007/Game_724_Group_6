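; BP_ButtonTarget_Overlap is a one-shot button that deactivates a linked target wall when an actor tagged Pickup overlaps its hit box.
; The first such overlap latches Activated, then, if TargetWall is valid, calls DeactivateWall and the visual event.
; That event swaps the button mesh's material and plays a timeline whose update sets the mesh to a fixed lowered offset from its BeginPlay location.
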(event OnComponentBeginOverlap(HitBox)
  (params (OverlappedComponent :type Primitive%20Component%20Object%20Reference) (OtherActor :type Actor%20Object%20Reference) (OtherComp :type Primitive%20Component%20Object%20Reference) (OtherBodyIndex :type Integer) (bFromSweep :type Boolean) (SweepResult :type Hit%20Result%20Structure%20%28by%20ref%29))
  (if (not (Variables|Default|GetbActivated))
    (if (Actor|ActorHasTag OtherActor "Pickup")
      (Variables|Default|SetbActivated true)
      (Utilities|IsValid (Variables|Default|GetTargetWall)
        (:Is%20Valid
          (Default|DeactivateWall (Variables|Default|GetTargetWall))
          (CallFunction|ActiveButtonVisual))))))

(event Custom|ActiveButtonVisual
  (Rendering|Material|SetMaterial (Variables|Default|GetButtonMesh) 0 "/Engine/EngineMeshes/BackgroundMaterial.BackgroundMaterial")
  (Timeline|Timeline Play
    (:Update
      (Transformation|SetRelativeLocation (Variables|Default|GetButtonMesh) (- (Variables|Default|GetStartButtonLocation) "0.000000,0.000000,50.000000") false false))))

(event EventBeginPlay
  (Variables|Default|SetStartButtonLocation (Variables|/Script/Engine.SceneComponent|GetRelativeLocation (Variables|Default|GetButtonMesh))))

(event Collision|EventActorBeginOverlap
  (params (OtherActor :type Actor%20Object%20Reference)))

(event EventTick
  (params (DeltaSeconds :type Float%20%28single-precision%29)))

(fn ConstructionScript)