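; Grid puzzle manager that flashes random target cells and deactivates a linked wall once enough pattern hits register.
; On BeginPlay it resets its cells, hands them a self-reference, marks pattern cells and starts a looping timer.
; Each tick of that timer targets a random managed cell, ignoring the non-activated list it builds.
; RegesterPatternHit counts hits up to the pattern size, then SolvePuzzle stops flashing and clears targets.
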(event EventBeginPlay
  (Variables|Default|SetActivatedCount 0)
  (Variables|Default|SetRequiredActivatedCount (Utilities|Array|Length (Variables|Default|GetPatternCells)))
  (for _array_element (Variables|Default|GetManageCells)
    (Variables|/Game/PreLevel/BP/Bp_GridCell_Pattern.Bp_GridCell_Pattern_C|SetGridManagerRef _array_element self)
    (Variables|/Game/PreLevel/BP/Bp_GridCell_Pattern.Bp_GridCell_Pattern_C|SetbIsActivated _array_element false)
    (Variables|/Game/PreLevel/BP/Bp_GridCell_Pattern.Bp_GridCell_Pattern_C|SetbIsCurrentTarget _array_element false)
    (Variables|/Game/PreLevel/BP/Bp_GridCell_Pattern.Bp_GridCell_Pattern_C|SetbIsLit _array_element false)
    (Variables|/Game/PreLevel/BP/Bp_GridCell_Pattern.Bp_GridCell_Pattern_C|SetbIsPatternCell _array_element false)
    (Default|UpdateVisual _array_element))
  (for _array_element_2 (Variables|Default|GetPatternCells)
    (Variables|/Game/PreLevel/BP/Bp_GridCell_Pattern.Bp_GridCell_Pattern_C|SetbIsPatternCell _array_element_2 true))
  (CallFunction|StartFlashing))

(event Collision|EventActorBeginOverlap
  (params (OtherActor :type Actor%20Object%20Reference)))

(event EventTick
  (params (DeltaSeconds :type Float%20%28single-precision%29)))

(fn ConstructionScript)

(fn StartFlashing
  (bind _returnvalue (Utilities|Time|SetTimerbyFunctionName 0 "AdvanceLitCell" (Variables|Default|GetFlashInterval) true))
  (Variables|Default|SetFlashTimerHandle _returnvalue)
  (CallFunction|AdvanceLitCell))

(fn AdvanceLitCell
  (if (not (Variables|Default|GetbPuzzleSolved))
    (Utilities|Array|Clear (Variables|Default|GetAvalilableCells))
    (for _array_element (Variables|Default|GetManageCells)
      (Default|SetasCurrentTarget _array_element false)
      (for _array_element_2 (Variables|Default|GetManageCells)
        (if (not (Variables|/Game/PreLevel/BP/Bp_GridCell_Pattern.Bp_GridCell_Pattern_C|GetbIsActivated _array_element_2))
          (Utilities|Array|Add (Variables|Default|GetAvalilableCells) _array_element_2))))
    (Default|SetasCurrentTarget (Utilities|Array|Get(acopy) (Variables|Default|GetManageCells) (Math|Random|RandomIntegerinRange 0 (- (Utilities|Array|Length (Variables|Default|GetManageCells)) 1))) true)))

(fn SolvePuzzle
  (bind _wallref (Variables|Default|GetWallRef))
  (Variables|Default|SetbPuzzleSolved true)
  (CallFunction|StopFlashing)
  (for _array_element (Variables|Default|GetManageCells)
    (Default|SetasCurrentTarget _array_element false))
  (Utilities|IsValid _wallref
    (:Is%20Valid
      (Default|DeactivateWall _wallref))))

(fn RegesterPatternHit
  (params (HitCell :type Bp%20Grid%20Cell%20Pattern%20Object%20Reference))
  (bind _output_get (Variables|Default|SetActivatedCount (+ (Variables|Default|GetActivatedCount) 1)))
  (if (>= _output_get (Variables|Default|GetRequiredActivatedCount))
    (CallFunction|SolvePuzzle)))

(fn StopFlashing
  (Utilities|Time|ClearandInvalidateTimerbyHandle (Variables|Default|GetFlashTimerHandle)))