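; Grid puzzle manager that lights one random cell at a time as the current target until the puzzle is solved.
; On BeginPlay it gives each managed cell a reference to itself and starts a looping timer.
; Each timer tick clears all targets and picks a random one, which can repeat the previous cell.
; SolvePuzzle, not called within this Blueprint, stops the timer and deactivates the linked wall.
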(event EventBeginPlay
  (for _array_element (Variables|Default|GetManageCells)
    (Variables|/Game/PreLevel/BP/Bp_GridCell.Bp_GridCell_C|SetGridManagerRef _array_element self))
  (CallFunction|StartFlashing))

(event Collision|EventActorBeginOverlap
  (params (OtherActor :type Actor%20Object%20Reference)))

(event EventTick
  (params (DeltaSeconds :type Float%20%28single-precision%29)))

(fn ConstructionScript)

(fn StartFlashing
  (bind _returnvalue (Utilities|Time|SetTimerbyFunctionName 0 "AdvanceLitCell" (Variables|Default|GetFlashInterval) true))
  (Variables|Default|SetFlashTimerHandle _returnvalue)
  (CallFunction|AdvanceLitCell))

(fn AdvanceLitCell
  (if (not (Variables|Default|GetbPuzzleSolved))
    (for _array_element (Variables|Default|GetManageCells)
      (Default|SetasCurrentTarget _array_element false))
    (Default|SetasCurrentTarget (Utilities|Array|Get(acopy) (Variables|Default|GetManageCells) (Math|Random|RandomIntegerinRange 0 (- (Utilities|Array|Length (Variables|Default|GetManageCells)) 1))) true)))

(fn SolvePuzzle
  (bind _wallref (Variables|Default|GetWallRef))
  (Variables|Default|SetbPuzzleSolved true)
  (Utilities|Time|ClearandInvalidateTimerbyHandle (Variables|Default|GetFlashTimerHandle))
  (Utilities|IsValid _wallref
    (:Is%20Valid
      (Default|DeactivateWall _wallref))))