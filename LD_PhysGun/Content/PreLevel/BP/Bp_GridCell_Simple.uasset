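; Grid cell actor for a puzzle, showing normal, lit or activated state by swapping its mesh material.
; Its functions mark it as the current target, which lights it, or activate it, which clears the lit state.
; When a BP_DataBlock hits its HitBox while it is the target and the grid manager reference is valid, it tells the manager to solve the puzzle and starts the block's absorb.
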(event OnComponentBeginOverlap(HitBox)
  (params (OverlappedComponent :type Primitive%20Component%20Object%20Reference) (OtherActor :type Actor%20Object%20Reference) (OtherComp :type Primitive%20Component%20Object%20Reference) (OtherBodyIndex :type Integer) (bFromSweep :type Boolean) (SweepResult :type Hit%20Result%20Structure%20%28by%20ref%29)))

(event OnComponentHit(HitBox)
  (params (HitComponent :type Primitive%20Component%20Object%20Reference) (OtherActor :type Actor%20Object%20Reference) (OtherComp :type Primitive%20Component%20Object%20Reference) (NormalImpulse :type Vector :default "0, 0, 0") (Hit :type Hit%20Result%20Structure%20%28by%20ref%29))
  (bind _asbp_data_block (Utilities|Casting|CastToBP_DataBlock OtherActor))
  (Variables|Default|SetBP%20Data%20Block _asbp_data_block)
  (Utilities|IsValid (Variables|Default|GetGridManagerRef)
    (:Is%20Valid
      (if (Variables|Default|GetbIsCurrentTarget)
        (Default|SolvePuzzle (Variables|Default|GetGridManagerRef))
        (Default|StartAbsorb (Variables|Default|GetBP%20Data%20Block) "0, 0, 0")))))

(event EventBeginPlay
  (CallFunction|UpdateVisual))

(event Collision|EventActorBeginOverlap
  (params (OtherActor :type Actor%20Object%20Reference)))

(event EventTick
  (params (DeltaSeconds :type Float%20%28single-precision%29)))

(fn ConstructionScript)

(fn UpdateVisual
  (if (Variables|Default|GetbIsActivated)
    (Rendering|Material|SetMaterial (Variables|Default|GetCellMesh) 0 (Variables|Default|GetActivatedMat))
    (elif (Variables|Default|GetbIsLit)
      (Rendering|Material|SetMaterial (Variables|Default|GetCellMesh) 0 (Variables|Default|GetLitMat))
      (else
        (Rendering|Material|SetMaterial (Variables|Default|GetCellMesh) 0 (Variables|Default|GetNormalMat))))))

(fn SetLitState
  (params (NewLitState :type Boolean))
  (Variables|Default|SetbIsLit NewLitState)
  (CallFunction|UpdateVisual))

(fn ActivateCell
  (Variables|Default|SetbIsActivated true)
  (Variables|Default|SetbIsLit false)
  (CallFunction|UpdateVisual))

(fn SetasCurrentTarget
  (params (NewIsTarget :type Boolean))
  (Variables|Default|SetbIsCurrentTarget NewIsTarget)
  (CallFunction|SetLitState NewIsTarget))