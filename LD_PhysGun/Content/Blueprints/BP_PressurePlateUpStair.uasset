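; Pressure plate that completes a Level 2 puzzle when an actor tagged "Pickup" enters its box.
; The overlap highlights the object via custom depth and stops its physics, then once only plays a sound, attaches it to the ring, moves its mesh and removes the tag.
; It then plays the finished-puzzle level sequence with player input disabled and player hidden, blending the view back to the pawn afterwards.
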(event OnComponentBeginOverlap(Box)
  (params (OverlappedComponent :type Primitive%20Component%20Object%20Reference) (OtherActor :type Actor%20Object%20Reference) (OtherComp :type Primitive%20Component%20Object%20Reference) (OtherBodyIndex :type Integer) (bFromSweep :type Boolean) (SweepResult :type Hit%20Result%20Structure%20%28by%20ref%29))
  (bind _returnvalue (Actor|GetComponentbyClass OtherActor "/Script/Engine.StaticMeshComponent"))
  (if (Actor|ActorHasTag OtherActor "Pickup")
    (Rendering|SetRenderCustomDepth _returnvalue true)
    (Physics|SetSimulatePhysics _returnvalue false)
    (Utilities|FlowControl|DoOnce false
      (:Completed
        (Audio|PlaySoundatLocation "/Game/Audio/CoinPickup.CoinPickup" "0, 0, 0" "0, 0, 0" 1.0 1.0 0.0 0 0 0 0)
        (Transformation|AttachComponentToComponent OtherActor (Variables|Default|GetSuperGrid_RingFull) "None" "KeepWorld" "KeepWorld" "KeepWorld" false)
        (Components|MoveComponentTo _returnvalue "0.000000,0.000000,400.000000" "0, 0, 0" true true 1.0 false)
        (Utilities|Array|RemoveItem (Variables|/Script/Engine.Actor|GetTags OtherActor) "Pickup")
        (Utilities|FlowControl|DoOnce false
          (:Completed
            (bind _outactor (Sequencer|Player|CreateLevelSequencePlayer "/Game/LevelSquence/LSQ_Level2_FinishedPuzzle.LSQ_Level2_FinishedPuzzle" (Utilities|Struct|MakeMovieSceneSequencePlaybackSettings false "(Value=0)" "(TickIntervalSeconds=0.000000,EvaluationBudgetMicroseconds=0.000000,bTickWhenPaused=False,bAllowRounding=True)" 1.0 0.0 false true true true false false "ForceKeepState" false)))
            (Sequencer|Player|Play (Variables|/Script/LevelSequence.LevelSequenceActor|GetSequencePlayer _outactor) :!class /Script/MovieScene.MovieSceneSequencePlayer)
            (EventDispatchers|BindEventtoOnFinished (Variables|/Script/LevelSequence.LevelSequenceActor|GetSequencePlayer _outactor) (delegate Custom|OnFinished))))))))

(event Custom|OnFinished
  (Game|Player|SetViewTargetwithBlend (Game|GetPlayerController 0) (Game|Player|GetPlayerPawn 0) 0.0 "VTBlend_Linear" 0.0 false))

(event EventBeginPlay
  (Utilities|IsValid (Variables|Default|GetTargetActor)
    (:Is%20Valid
      (Variables|Default|SetFinalLocation (+ (Transformation|GetActorLocation) (Variables|Default|GetTarget%20Relative%20Location))))))

(event Collision|EventActorBeginOverlap
  (params (OtherActor :type Actor%20Object%20Reference)))

(event EventTick
  (params (DeltaSeconds :type Float%20%28single-precision%29)))

(fn ConstructionScript)