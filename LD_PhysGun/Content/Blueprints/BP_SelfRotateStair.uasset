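; Staircase actor that swings its mesh back and forth in yaw through roughly a quarter turn on its own.
; Tick rotates the mesh at RotationSpeed, pausing briefly at each limit before reversing, with DoOnce gates limiting the mechanism sound to once per swing.
; RemoteToggleDirection flips direction on demand and temporarily enables a custom depth stencil on the mesh.
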(event EventBeginPlay)

(event Collision|EventActorBeginOverlap
  (params (OtherActor :type Actor%20Object%20Reference)))

(event EventTick
  (params (DeltaSeconds :type Float%20%28single-precision%29))
  (if (not (Variables|Default|GetIswaiting))
    (Utilities|FlowControl|Sequence
      (:then_0
        (Utilities|FlowControl|DoOnce false :!label _label
          (:Completed
            (Audio|PlaySoundatLocation "/Game/Audio/Complex-mechanism-long.Complex-mechanism-long" (Transformation|GetActorLocation) "0, 0, 0" 1.0 1.0 0.0 "/Game/Audio/Level2_AudioDecrease.Level2_AudioDecrease" 0 0 0))))
      (:then_1
        (Transformation|AddRelativeRotation (Variables|Default|GetStaticMesh) (Math|Rotator|MakeRotator 0.0 0.0 (* (* DeltaSeconds (Variables|Default|GetRotationSpeed)) (select (Variables|Default|GetIsRevered) 1.0 -1.0))) false false)
        (if (or (and (>= (.yaw (Variables|/Script/Engine.SceneComponent|GetRelativeRotation (Variables|Default|GetStaticMesh))) 179.0) (== (Variables|Default|GetIsRevered) true)) (and (<= (.yaw (Variables|/Script/Engine.SceneComponent|GetRelativeRotation (Variables|Default|GetStaticMesh))) 91.0) (== (Variables|Default|GetIsRevered) false)))
          (Variables|Default|SetIswaiting true)
          (Utilities|FlowControl|DoOnce false :!label _label_2
            (:Completed
              (Utilities|FlowControl|Delay 2.0)
              (Variables|Default|SetIsRevered (not (Variables|Default|GetIsRevered)))
              (Variables|Default|SetIswaiting false)
              (Utilities|FlowControl|Sequence
                (:then_0
                  (goto _label_2 Reset))
                (:then_1
                  (goto _label Reset))))))))))

(event EventRemoteToggleDirection
  (bind _staticmesh (Variables|Default|GetStaticMesh))
  (Variables|Default|SetIsRevered (not (Variables|Default|GetIsRevered)))
  (Rendering|SetRenderCustomDepth _staticmesh true)
  (Rendering|SetCustomDepthStencilValue _staticmesh 1)
  (Utilities|FlowControl|Delay 5.0)
  (Rendering|SetRenderCustomDepth _staticmesh false)
  (Rendering|SetCustomDepthStencilValue _staticmesh 0))

(fn ConstructionScript)