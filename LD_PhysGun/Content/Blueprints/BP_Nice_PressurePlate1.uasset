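; Pressure plate actor that reacts when a tagged pickup object enters its Test trigger volume.
; An overlapping actor with both the Pickup and Detact tags sets Test1 on the first BP_Nice_Ball found, prints a debug message and turns on the plate's custom depth rendering.
; Any end overlap turns custom depth off without checking tags, and Test1 stays set.
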(event OnComponentBeginOverlap(Test)
  (params (OverlappedComponent :type Primitive%20Component%20Object%20Reference) (OtherActor :type Actor%20Object%20Reference) (OtherComp :type Primitive%20Component%20Object%20Reference) (OtherBodyIndex :type Integer) (bFromSweep :type Boolean) (SweepResult :type Hit%20Result%20Structure%20%28by%20ref%29))
  (if (Actor|ActorHasTag OtherActor "Pickup")
    (if (Actor|ActorHasTag OtherActor "Detact")
      (bind _returnvalue (Actor|GetActorOfClass "/Game/Blueprints/BP_Nice_Ball.BP_Nice_Ball_C"))
      (Variables|/Game/Blueprints/BP_Nice_Ball.BP_Nice_Ball_C|SetTest_1 _returnvalue true)
      (Development|PrintString "1")
      (Rendering|SetRenderCustomDepth (Variables|Default|GetPlate) true))))

(event OnComponentEndOverlap(Test)
  (params (OverlappedComponent :type Primitive%20Component%20Object%20Reference) (OtherActor :type Actor%20Object%20Reference) (OtherComp :type Primitive%20Component%20Object%20Reference) (OtherBodyIndex :type Integer))
  (Rendering|SetRenderCustomDepth (Variables|Default|GetPlate) false))

(fn ConstructionScript)