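; BP_NiceRotateObject is an actor that boosts components entering its Box trigger along the forward direction of its StaticMesh.
; On overlap begin it applies a velocity-change impulse to the other component, scaled by BoostStrength, so mass is ignored.
; EnableHighLight and DisableHighLight events toggle the mesh's custom depth rendering for highlighting.
; Despite the name, the graphs contain no rotation logic.
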(event OnComponentBeginOverlap(Box)
  (params (OverlappedComponent :type Primitive%20Component%20Object%20Reference) (OtherActor :type Actor%20Object%20Reference) (OtherComp :type Primitive%20Component%20Object%20Reference) (OtherBodyIndex :type Integer) (bFromSweep :type Boolean) (SweepResult :type Hit%20Result%20Structure%20%28by%20ref%29))
  (Physics|AddImpulse OtherComp (* (Math|Vector|GetForwardVector (Variables|Default|GetStaticMesh)) (Variables|Default|GetBoostStrength)) "None" true))

(event Custom|DisableHighLight
  (Rendering|SetRenderCustomDepth (Variables|Default|GetStaticMesh) false))

(event Custom|EnableHighLight
  (Rendering|SetRenderCustomDepth (Variables|Default|GetStaticMesh) true))

(fn ConstructionScript)