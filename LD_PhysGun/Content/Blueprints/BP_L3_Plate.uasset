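; BP_L3_Plate is a Level 3 pressure plate that reports to a linked door when pickup cubes rest on it.
; Box overlap events count only BP_L3_PickupCube actors.
; The first cube to enter calls AddPlate on LinkedDoor and the last to leave calls RemovePlate, so several cubes on one plate register as a single press.
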(event OnComponentBeginOverlap(Box)
  (params (OverlappedComponent :type Primitive%20Component%20Object%20Reference) (OtherActor :type Actor%20Object%20Reference) (OtherComp :type Primitive%20Component%20Object%20Reference) (OtherBodyIndex :type Integer) (bFromSweep :type Boolean) (SweepResult :type Hit%20Result%20Structure%20%28by%20ref%29))
  (Utilities|Casting|CastToBP_L3_PickupCube OtherActor)
  (Variables|Default|SetOverlappingObjects (+ (Variables|Default|GetOverlappingObjects) 1))
  (if (== (Variables|Default|GetOverlappingObjects) 1)
    (Default|AddPlate (Variables|Default|GetLinkedDoor))))

(event OnComponentEndOverlap(Box)
  (params (OverlappedComponent :type Primitive%20Component%20Object%20Reference) (OtherActor :type Actor%20Object%20Reference) (OtherComp :type Primitive%20Component%20Object%20Reference) (OtherBodyIndex :type Integer))
  (Utilities|Casting|CastToBP_L3_PickupCube OtherActor)
  (Variables|Default|SetOverlappingObjects (- (Variables|Default|GetOverlappingObjects) 1))
  (if (== (Variables|Default|GetOverlappingObjects) 0)
    (Default|RemovePlate (Variables|Default|GetLinkedDoor))))

(fn ConstructionScript)