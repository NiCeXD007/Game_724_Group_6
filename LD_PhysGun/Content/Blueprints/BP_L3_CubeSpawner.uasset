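; BP_L3_CubeSpawner spawns pickup cubes where the first-person camera is aimed when E is pressed.
; A Visibility line trace runs 2000 units forward from the camera.
; On a blocking hit whose actor lacks the "CubeSpawner" tag, it spawns a BP_L3_PickupCube above the impact location.
; Actors carrying that tag are excluded as spawn targets, and the construction script is empty.
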(event Input|KeyboardEvents|E
  (params (Key :type Key%20Structure :default "None"))
  (bind _firstpersoncamera (Variables|Default|GetFirstPersonCamera))
  (bind _returnvalue (Transformation|GetWorldLocation _firstpersoncamera))
  (:Pressed
    (bind _outhit (Collision|LineTraceByChannel _returnvalue (+ _returnvalue (* (Math|Vector|GetForwardVector (Variables|Default|GetFirstPersonCamera)) 2000)) "TraceTypeQuery1" false 0 "None"))
    (if (not (Actor|ActorHasTag (.HitActor (Collision|BreakHitResult _outhit)) "CubeSpawner"))
      (if (.bBlockingHit (Collision|BreakHitResult _outhit))
        (Game|SpawnActorfromClass "/Game/Blueprints/BP_L3_PickupCube.BP_L3_PickupCube_C" (Math|Transform|MakeTransform (+ (.Location (Collision|BreakHitResult _outhit)) "0.000000,0.000000,200.000000") "0, 0, 0" "1.000000,1.000000,1.000000") "Undefined" "MultiplyWithRoot" 0 0)))))

(fn ConstructionScript)