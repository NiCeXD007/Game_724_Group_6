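; Door Blueprint that swings its Box component a quarter turn on overlap, gated by a flag from BP_Nice_CubeTest.
; Tick looks up that actor and copies its Check value into EngCheck.
; A Box begin overlap with EngCheck set makes Box movable, then a DoOnce rotates it and sets SuperGridBoxCentered static.
; End overlap restores Box's zero rotation and resets the DoOnce, regardless of the flag.
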(event OnComponentBeginOverlap(Box)
  (params (OverlappedComponent :type Primitive%20Component%20Object%20Reference) (OtherActor :type Actor%20Object%20Reference) (OtherComp :type Primitive%20Component%20Object%20Reference) (OtherBodyIndex :type Integer) (bFromSweep :type Boolean) (SweepResult :type Hit%20Result%20Structure%20%28by%20ref%29))
  (if (Variables|Default|GetEngCheck)
    (Transformation|SetMobility (Variables|Default|GetBox) "Movable")
    (Utilities|FlowControl|DoOnce false
      (:Completed
        (Transformation|SetRelativeRotation (Variables|Default|GetBox) "0.000000,-90.000000,0.000000" false false)
        (Transformation|SetMobility (Variables|Default|GetSuperGrid_BoxCentered) "Static")))))

(event OnComponentEndOverlap(Box)
  (params (OverlappedComponent :type Primitive%20Component%20Object%20Reference) (OtherActor :type Actor%20Object%20Reference) (OtherComp :type Primitive%20Component%20Object%20Reference) (OtherBodyIndex :type Integer))
  (Transformation|SetMobility (Variables|Default|GetBox) "Movable")
  (Transformation|SetRelativeRotation (Variables|Default|GetBox) "0.000000,0.000000,0.000000" false false)
  (Utilities|FlowControl|DoOnce false) ; enters at Reset
)

(event EventTick
  (params (DeltaSeconds :type Float%20%28single-precision%29))
  (bind _returnvalue (Actor|GetActorOfClass "/Game/Blueprints/BP_Nice_CubeTest.BP_Nice_CubeTest_C"))
  (Variables|Default|SetEngCheck (Variables|/Game/Blueprints/BP_Nice_CubeTest.BP_Nice_CubeTest_C|GetCheck _returnvalue)))

(fn ConstructionScript)