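; BP_L3_BridgeRotator is an actor that rotates a referenced TargetRotate actor, presumably a bridge, when TriggerRotation is called.
; It takes its own rotation, not the target's, as the start and adds 90 degrees of yaw, wrapped at 360, for the end.
; A timeline lerps the target between the two, while an IsRotating flag blocks retriggers until it finishes.
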(event Custom|TriggerRotation
  (bind _targetrotate (Variables|Default|GetTargetRotate))
  (if (not (Variables|Default|GetisRotating))
    (Utilities|IsValid _targetrotate
      (:Is%20Valid
        (Variables|Default|SetStartRotation (.Rotation (Math|Transform|BreakTransform (Transformation|GetActorTransform))))
        (Variables|Default|SetEndRotation (Math|Rotator|MakeRotator (.Roll (Math|Rotator|BreakRotator (Variables|Default|GetStartRotation))) (.Pitch (Math|Rotator|BreakRotator (Variables|Default|GetStartRotation))) (Math|Float|%(Float) (+ (.Yaw (Math|Rotator|BreakRotator (Variables|Default|GetStartRotation))) 9e+01) 3.6e+02)))
        (Variables|Default|SetisRotating true)
        (bind _newtrack_0 (Timeline|Timeline PlayFromStart)
          (:Update
            (Transformation|SetActorRotation _targetrotate (Math|Rotator|Lerp(Rotator) (Variables|Default|GetStartRotation) (Variables|Default|GetEndRotation) _newtrack_0)))
          (:Finished
            (Variables|Default|SetisRotating false)))))))

(fn ConstructionScript)