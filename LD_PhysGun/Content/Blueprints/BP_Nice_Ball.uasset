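; BP_Nice_Ball is a Blueprint that appears to be a test for swapping its static mesh for an oversized ball.
; An event track on the SpawnBall timeline passes three nested Test checks and a DoOnce, then adds a scaled-up mesh component, stores it as Ball and destroys the original StaticMesh.
; Nothing starts the timeline, so this logic never runs, and the construction script is empty.
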(fn ConstructionScript)