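; BP_SelfRotateDoor is a door actor that continuously swings back and forth over roughly a half turn of yaw.
; Tick rotates the StaticMesh at RotationSpeed in the direction set by IsRevered, pausing briefly at each limit before flipping it.
; RemoteToggleDirection reverses the swing on demand and temporarily enables custom depth with a stencil value on the mesh.
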(event EventBeginPlay)

(event Collision|EventActorBeginOverlap
  (params (OtherActor :type Actor%20Object%20Reference)))

(event EventTick
  (params (DeltaSeconds :type Float%20%28single-precision%29))
  (if (not (Variables|Default|GetIswaiting))
    (Transformation|AddRelativeRotation (Variables|Default|GetStaticMesh) (Math|Rotator|MakeRotator 0.0 0.0 (* (* DeltaSeconds (Variables|Default|GetRotationSpeed)) (select (Variables|Default|GetIsRevered) 1.0 -1.0))) false false)
    (if (or (and (>= (.yaw (Variables|/Script/Engine.SceneComponent|GetRelativeRotation (Variables|Default|GetStaticMesh))) 179.0) (== (Variables|Default|GetIsRevered) true)) (and (<= (.yaw (Variables|/Script/Engine.SceneComponent|GetRelativeRotation (Variables|Default|GetStaticMesh))) 1.0) (== (Variables|Default|GetIsRevered) false)))
      (Variables|Default|SetIswaiting true)
      (Utilities|FlowControl|DoOnce false :!label _label
        (:Completed
          (Utilities|FlowControl|Delay 1.0)
          (Variables|Default|SetIsRevered (not (Variables|Default|GetIsRevered)))
          (Variables|Default|SetIswaiting false)
          (goto _label Reset))))))

(event EventRemoteToggleDirection
  (bind _staticmesh (Variables|Default|GetStaticMesh))
  (Variables|Default|SetIsRevered (not (Variables|Default|GetIsRevered)))
  (Rendering|SetRenderCustomDepth _staticmesh true)
  (Rendering|SetCustomDepthStencilValue _staticmesh 1)
  (Utilities|FlowControl|Delay 5.0)
  (Rendering|SetRenderCustomDepth _staticmesh false)
  (Rendering|SetCustomDepthStencilValue _staticmesh 0))

(fn ConstructionScript)