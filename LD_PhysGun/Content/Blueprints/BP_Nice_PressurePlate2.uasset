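; BP_Nice_PressurePlate2 is a pressure plate that reacts when an actor tagged both Pickup and Detact overlaps its Test component.
; It finds a BP_Nice_Ball in the level, briefly sets that ball's Test2 flag and turns on the Plate's custom depth rendering.
; After a short delay it resets both, rather than waiting for the overlap to end, with debug prints marking each step.
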(event OnComponentBeginOverlap(Test)
  (params (OverlappedComponent :type Primitive%20Component%20Object%20Reference) (OtherActor :type Actor%20Object%20Reference) (OtherComp :type Primitive%20Component%20Object%20Reference) (OtherBodyIndex :type Integer) (bFromSweep :type Boolean) (SweepResult :type Hit%20Result%20Structure%20%28by%20ref%29))
  (if (Actor|ActorHasTag OtherActor "Pickup")
    (if (Actor|ActorHasTag OtherActor "Detact")
      (bind _returnvalue (Actor|GetActorOfClass "/Game/Blueprints/BP_Nice_Ball.BP_Nice_Ball_C"))
      (Variables|/Game/Blueprints/BP_Nice_Ball.BP_Nice_Ball_C|SetTest_2 _returnvalue true)
      (Development|PrintString "2?")
      (Rendering|SetRenderCustomDepth (Variables|Default|GetPlate) true)
      (Utilities|FlowControl|Delay 0.9)
      (Variables|/Game/Blueprints/BP_Nice_Ball.BP_Nice_Ball_C|SetTest_2 _returnvalue false)
      (Rendering|SetRenderCustomDepth (Variables|Default|GetPlate) false)
      (Development|PrintString "2!"))))

(fn ConstructionScript)