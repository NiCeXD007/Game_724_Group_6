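; BP_RotateObject is an actor with a static mesh that can be highlighted; despite its name, the file contains no rotation logic.
; EnableHighLight turns on Custom Depth rendering with a stencil value for outline-style effects, but only when the mesh is Movable; otherwise it calls DisableHighLight.
; DisableHighLight turns Custom Depth off and clears the stencil.
; BeginPlay, overlap, Tick and the construction script are empty.
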(event Custom|DisableHighLight
  (bind _staticmesh (Variables|Default|GetStaticMesh))
  (Rendering|SetRenderCustomDepth _staticmesh false)
  (Rendering|SetCustomDepthStencilValue _staticmesh 0))

(event Custom|EnableHighLight
  (bind _staticmesh (Variables|Default|GetStaticMesh))
  (if (Utilities|Enum|Equal(Enum) (Variables|/Script/Engine.SceneComponent|GetMobility _staticmesh) "Movable")
    (Rendering|SetRenderCustomDepth _staticmesh true)
    (Rendering|SetCustomDepthStencilValue _staticmesh 1)
    (else
      (CallFunction|DisableHighLight))))

(event EventBeginPlay)

(event Collision|EventActorBeginOverlap
  (params (OtherActor :type Actor%20Object%20Reference)))

(event EventTick
  (params (DeltaSeconds :type Float%20%28single-precision%29)))

(fn ConstructionScript)