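; Level 3 trigger that plays a cutscene once enough plates are active.
; AddPlate counts up and, at the Trigger threshold, blocks move input, starts a delayed camera shake, then through a DoOnce plays TargetSequence, hides the pawn and rotates the mesh by Timeline.
; RemovePlate reverses the rotation when the count drops below the threshold.
; The sequence's finish event unhides the pawn and restores movement.
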(event Custom|AddPlate
  (Variables|Default|Setactiveplates (+ (Variables|Default|Getactiveplates) 1))
  (if (>= (Variables|Default|Getactiveplates) (Variables|Default|GetTrigger))
    (Input|SetIgnoreMoveInput (Game|GetPlayerController 0) true)
    (Utilities|FlowControl|Delay 1.5)
    (CameraShakes|StartCameraShake (Game|GetPlayerCameraManager 0) "/Game/Blueprints/CS_L3_CameraShake.CS_L3_CameraShake_C" 1.0 "CameraLocal" "0, 0, 0")
    (Utilities|FlowControl|Delay 7.0)
    (Utilities|FlowControl|DoOnce false
      (:Completed
        (Sequencer|Player|Play (Variables|/Script/LevelSequence.LevelSequenceActor|GetSequencePlayer (Variables|Default|GetTargetSequence)) :!class /Script/MovieScene.MovieSceneSequencePlayer)
        (Rendering|SetActorHiddenInGame (Game|Player|GetPlayerPawn 0) true)
        (bind _newtrack_0 (Timeline|Timeline Play)
          (:Update
            (Transformation|SetRelativeRotation (Variables|Debug|GetStaticMeshComponent) (Math|Rotator|Lerp(Rotator) "90.000000,0.000000,0.000000" "90.000000,90.000000,0.000000" _newtrack_0) false false)
            (EventDispatchers|AssignOnFinished (Variables|/Script/LevelSequence.LevelSequenceActor|GetSequencePlayer (Variables|Default|GetTargetSequence)) (delegate Custom|OnFinished_Event))))))))

(event Custom|RemovePlate
  (Variables|Default|Setactiveplates (- (Variables|Default|Getactiveplates) 1))
  (if (< (Variables|Default|Getactiveplates) (Variables|Default|GetTrigger))
    (bind _newtrack_0 (Timeline|Timeline Reverse)
      (:Update
        (Transformation|SetRelativeRotation (Variables|Debug|GetStaticMeshComponent) (Math|Rotator|Lerp(Rotator) "90.000000,0.000000,0.000000" "90.000000,90.000000,0.000000" _newtrack_0) false false)
        (EventDispatchers|AssignOnFinished (Variables|/Script/LevelSequence.LevelSequenceActor|GetSequencePlayer (Variables|Default|GetTargetSequence)) (delegate Custom|OnFinished_Event))))))

(event Custom|OnFinished_Event
  (Development|PrintString "Hello")
  (Rendering|SetActorHiddenInGame (Game|Player|GetPlayerPawn 0) false)
  (Input|SetIgnoreMoveInput (Game|GetPlayerController 0) false))

(fn ConstructionScript)