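; BP_L3_DoorAnim1 is a Level 3 door that opens once enough plates are active.
; AddPlate and RemovePlate adjust an active plate count, and AddPlate prints the new value.
; When AddPlate brings the count to the Trigger threshold, it swaps the mesh to a holo material and plays a timeline that rotates it 90 degrees.
; RemovePlate never reverses the rotation or material change.
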(event Custom|AddPlate
  (bind _output_get (Variables|Default|Setactiveplates (+ (Variables|Default|Getactiveplates) 1)))
  (Development|PrintString (Utilities|String|ToString(Integer) _output_get))
  (if (>= (Variables|Default|Getactiveplates) (Variables|Default|GetTrigger))
    (Rendering|Material|SetMaterial (Variables|Debug|GetStaticMeshComponent) 0 "/Game/SuperGrid/TutorialLevel/MaterialInstances/M_L3_Tut_HoloD.M_L3_Tut_HoloD")
    (bind _newtrack_0 (Timeline|Timeline Play)
      (:Update
        (Transformation|SetRelativeRotation (Variables|Debug|GetStaticMeshComponent) (Math|Rotator|Lerp(Rotator) "90.000000,90.000000,0.000000" "90.000000,180.000000,0.000000" _newtrack_0) false false)))))

(event Custom|RemovePlate
  (Variables|Default|Setactiveplates (- (Variables|Default|Getactiveplates) 1))
  (if (< (Variables|Default|Getactiveplates) (Variables|Default|GetTrigger))
    _))

(fn ConstructionScript)