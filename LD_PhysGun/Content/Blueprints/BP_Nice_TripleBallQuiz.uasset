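; Triple-ball timing puzzle that opens BP_Nice_OpenDoor actors when all three trigger boxes register overlaps at nearly the same moment.
; BeginPlay starts three staggered timelines, whose Spawn events create BP_Nice_Ball actors above their boxes.
; Each overlap replays that box's timeline and raises its check flag for half a second, gated by a DoOnce.
; Tick polls the three flags and calls OpenTheDoor while all are true.
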(event OnComponentBeginOverlap(Box)
  (params (OverlappedComponent :type Primitive%20Component%20Object%20Reference) (OtherActor :type Actor%20Object%20Reference) (OtherComp :type Primitive%20Component%20Object%20Reference) (OtherBodyIndex :type Integer) (bFromSweep :type Boolean) (SweepResult :type Hit%20Result%20Structure%20%28by%20ref%29))
  (bind _box (Variables|Default|GetBox))
  (bind _returnvalue (Transformation|GetWorldLocation _box))
  ;[0.15 0.15 0.15 0.5] CheckAndRespawn
  (Utilities|FlowControl|Sequence
    (:then_0
      (Utilities|FlowControl|DoOnce false :!label _label
        (:Completed
          (Variables|Default|SetCheck_1 true)
          (Utilities|FlowControl|Delay 0.5)
          (Variables|Default|SetCheck_1 false)
          (goto _label Reset))))
    (:then_1
      (Timeline|BallSpawn_1 PlayFromStart
        (:SpawnEvent
          (Game|SpawnActorfromClass "/Game/Blueprints/BP_Nice_Ball.BP_Nice_Ball_C" (Math|Transform|MakeTransform (Math|Vector|MakeVector (.x _returnvalue) (.y _returnvalue) (+ (.z _returnvalue) 3.6e+02)) "0, 0, 0" "1.000000,1.000000,1.000000") "Undefined" "MultiplyWithRoot" 0 0))))))

(event OnComponentBeginOverlap(Box1)
  (params (OverlappedComponent :type Primitive%20Component%20Object%20Reference) (OtherActor :type Actor%20Object%20Reference) (OtherComp :type Primitive%20Component%20Object%20Reference) (OtherBodyIndex :type Integer) (bFromSweep :type Boolean) (SweepResult :type Hit%20Result%20Structure%20%28by%20ref%29))
  (bind _box1 (Variables|Default|GetBox1))
  (bind _returnvalue (Transformation|GetWorldLocation _box1))
  ;[0.15 0.15 0.15 0.5] CheckAndRespawn
  (Utilities|FlowControl|Sequence
    (:then_0
      (Utilities|FlowControl|DoOnce false :!label _label
        (:Completed
          (Variables|Default|SetCheck_2 true)
          (Utilities|FlowControl|Delay 0.5)
          (Variables|Default|SetCheck_2 false)
          (goto _label Reset))))
    (:then_1
      (Timeline|BallSpawn_2 PlayFromStart
        (:SpawnEvent
          (Game|SpawnActorfromClass "/Game/Blueprints/BP_Nice_Ball.BP_Nice_Ball_C" (Math|Transform|MakeTransform (Math|Vector|MakeVector (.x _returnvalue) (.y _returnvalue) (+ (.z _returnvalue) 3.6e+02)) "0, 0, 0" "1.000000,1.000000,1.000000") "Undefined" "MultiplyWithRoot" 0 0))))))

(event OnComponentBeginOverlap(Box2)
  (params (OverlappedComponent :type Primitive%20Component%20Object%20Reference) (OtherActor :type Actor%20Object%20Reference) (OtherComp :type Primitive%20Component%20Object%20Reference) (OtherBodyIndex :type Integer) (bFromSweep :type Boolean) (SweepResult :type Hit%20Result%20Structure%20%28by%20ref%29))
  (bind _box2 (Variables|Default|GetBox2))
  (bind _returnvalue (Transformation|GetWorldLocation _box2))
  ;[0.15 0.15 0.15 0.5] CheckAndRespawn
  (Utilities|FlowControl|Sequence
    (:then_0
      (Utilities|FlowControl|DoOnce false :!label _label
        (:Completed
          (Variables|Default|SetCheck_3 true)
          (Utilities|FlowControl|Delay 0.5)
          (Variables|Default|SetCheck_3 false)
          (goto _label Reset))))
    (:then_1
      (Timeline|BallSpawn_3 PlayFromStart
        (:SpawnEvent
          (Game|SpawnActorfromClass "/Game/Blueprints/BP_Nice_Ball.BP_Nice_Ball_C" (Math|Transform|MakeTransform (Math|Vector|MakeVector (.x _returnvalue) (.y _returnvalue) (+ (.z _returnvalue) 3.6e+02)) "0, 0, 0" "1.000000,1.000000,1.000000") "Undefined" "MultiplyWithRoot" 0 0))))))

(event EventTick
  (params (DeltaSeconds :type Float%20%28single-precision%29))
  ;[0.15 0.15 0.15 0.5] OpenTheDoor
  (if (Variables|Default|GetCheck_1)
    (if (Variables|Default|GetCheck_2)
      (if (Variables|Default|GetCheck_3)
        (bind _outactors (Actor|GetAllActorsOfClass "/Game/Blueprints/BP_Nice_OpenDoor.BP_Nice_OpenDoor_C"))
        (Default|OpentheDoor _outactors)))))

(event EventBeginPlay
  (bind _box (Variables|Default|GetBox))
  (bind _box1 (Variables|Default|GetBox1))
  (bind _box2 (Variables|Default|GetBox2))
  (bind _returnvalue (Transformation|GetWorldLocation _box))
  (bind _returnvalue_2 (Transformation|GetWorldLocation _box1))
  (bind _returnvalue_3 (Transformation|GetWorldLocation _box2))
  (Utilities|FlowControl|Sequence
    (:then_0
      ;[0.15 0.15 0.15 0.5] CheckAndRespawn
      (Timeline|BallSpawn_1 Play
        (:SpawnEvent
          (Game|SpawnActorfromClass "/Game/Blueprints/BP_Nice_Ball.BP_Nice_Ball_C" (Math|Transform|MakeTransform (Math|Vector|MakeVector (.x _returnvalue) (.y _returnvalue) (+ (.z _returnvalue) 3.6e+02)) "0, 0, 0" "1.000000,1.000000,1.000000") "Undefined" "MultiplyWithRoot" 0 0))))
    (:then_1
      (Utilities|FlowControl|Delay 1.0)
      (Timeline|BallSpawn_2 Play
        (:SpawnEvent
          (Game|SpawnActorfromClass "/Game/Blueprints/BP_Nice_Ball.BP_Nice_Ball_C" (Math|Transform|MakeTransform (Math|Vector|MakeVector (.x _returnvalue_2) (.y _returnvalue_2) (+ (.z _returnvalue_2) 3.6e+02)) "0, 0, 0" "1.000000,1.000000,1.000000") "Undefined" "MultiplyWithRoot" 0 0))))
    (:then_2
      (Utilities|FlowControl|Delay 2.0)
      (Timeline|BallSpawn_3 Play
        (:SpawnEvent
          (Game|SpawnActorfromClass "/Game/Blueprints/BP_Nice_Ball.BP_Nice_Ball_C" (Math|Transform|MakeTransform (Math|Vector|MakeVector (.x _returnvalue_3) (.y _returnvalue_3) (+ (.z _returnvalue_3) 3.6e+02)) "0, 0, 0" "1.000000,1.000000,1.000000") "Undefined" "MultiplyWithRoot" 0 0))))))

(fn ConstructionScript)