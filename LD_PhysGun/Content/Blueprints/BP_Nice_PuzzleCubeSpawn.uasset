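; Puzzle cube spawn actor that plays a one-time Level 4 detail cutscene and shoves whatever enters its box downward.
; The Letsgooo event destroys the Plane component once and plays the level sequence with player input disabled and the player hidden, keeping its end state.
; When the sequence finishes, the camera returns to the player pawn.
; Separately, box overlaps apply a strong downward velocity impulse to the entering component.
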(event OnComponentBeginOverlap(Box)
  (params (OverlappedComponent :type Primitive%20Component%20Object%20Reference) (OtherActor :type Actor%20Object%20Reference) (OtherComp :type Primitive%20Component%20Object%20Reference) (OtherBodyIndex :type Integer) (bFromSweep :type Boolean) (SweepResult :type Hit%20Result%20Structure%20%28by%20ref%29))
  (Physics|AddImpulse OtherComp "0.000000,0.000000,-2000.000000" "None" true))

(event Custom|Letsgooo
  (Utilities|FlowControl|DoOnce false
    (:Completed
      (Components|DestroyComponent (Variables|Default|GetPlane))
      (bind _outactor (Sequencer|Player|CreateLevelSequencePlayer "/Game/LevelSquence/LSQ_Level4_ForDetail.LSQ_Level4_ForDetail" (Utilities|Struct|MakeMovieSceneSequencePlaybackSettings false "(Value=0)" "(TickIntervalSeconds=0.000000,EvaluationBudgetMicroseconds=0.000000,bTickWhenPaused=False,bAllowRounding=True)" 1.0 0.0 false true true true false false "ForceKeepState" false)))
      (Sequencer|Player|Play (Variables|/Script/LevelSequence.LevelSequenceActor|GetSequencePlayer _outactor) :!class /Script/MovieScene.MovieSceneSequencePlayer)
      (EventDispatchers|BindEventtoOnFinished (Variables|/Script/LevelSequence.LevelSequenceActor|GetSequencePlayer _outactor) (delegate Custom|DetailEnd)))))

(event Custom|DetailEnd
  (Game|Player|SetViewTargetwithBlend (Game|GetPlayerController 0) (Game|Player|GetPlayerPawn 0) 0.0 "VTBlend_Linear" 0.0 false))

(fn ConstructionScript)