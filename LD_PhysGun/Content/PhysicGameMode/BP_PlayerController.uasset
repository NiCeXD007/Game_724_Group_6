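; BP_PlayerController is the player controller for the PhysicGameMode folder, handling the pause menu and level navigation.
; OpenPauseMenu creates a new WBP_PauseMenu, pauses the game, shows the cursor and switches to game-and-UI input, guarded by an open-state flag.
; ClosePauseMenu removes the widget and restores unpaused, game-only input.
; Separate events reload the current level by name or open LV_MainMenu.
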(event Custom|ClosePauseMenu
  (Utilities|IsValid (Variables|Default|GetPauseMenuRef)
    (:Is%20Valid
      (Widget|RemovefromParent (Variables|Default|GetPauseMenuRef))
      (Variables|Default|SetbIsPauseMenuOpen false)
      (Variables|Default|SetbShowMouseCursor false)
      (Game|SetGamePaused false)
      (Input|SetInputModeGameOnly self false))))

(event Custom|OpenPauseMenu
  (if (not (Variables|Default|GetbIsPauseMenuOpen))
    (bind _returnvalue (UserInterface|CreateWidget "/Game/UI/WBP_PauseMenu.WBP_PauseMenu_C" self))
    (bind _output_get (Variables|Default|SetPauseMenuRef _returnvalue))
    (UserInterface|Viewport|AddtoViewport _output_get 0)
    (Variables|Default|SetbIsPauseMenuOpen true)
    (Variables|Default|SetbShowMouseCursor true)
    (Input|SetInputModeGameandUI self (Variables|Default|GetPauseMenuRef) "DoNotLock" false false)
    (Game|SetGamePaused true)))

(event Custom|RestartCurrentLevel
  (bind _returnvalue (Game|GetCurrentLevelName true))
  (Game|OpenLevel(byName) (Utilities|String|StringToName _returnvalue)))

(event Custom|BackToMainMenu
  (Game|OpenLevel(byName) "LV_MainMenu"))

(event EventBeginPlay)

(event EventTick
  (params (DeltaSeconds :type Float%20%28single-precision%29)))

(fn ConstructionScript)