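; BP_L3_DoorAnim is a door that animates open while enough plates are active, likely pressure plates in level 3.
; AddPlate and RemovePlate adjust an active-plate count and compare it to a Trigger threshold.
; Reaching the threshold plays a Timeline that lerps the static mesh's relative rotation through a quarter turn.
; Dropping below it reverses the same Timeline to swing the mesh back.
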(event Custom|AddPlate
  (Variables|Default|Setactiveplates (+ (Variables|Default|Getactiveplates) 1))
  (if (>= (Variables|Default|Getactiveplates) (Variables|Default|GetTrigger))
    (bind _newtrack_0 (Timeline|Timeline Play)
      (:Update
        (Transformation|SetRelativeRotation (Variables|Debug|GetStaticMeshComponent) (Math|Rotator|Lerp(Rotator) "90.000000,0.000000,0.000000" "90.000000,90.000000,0.000000" _newtrack_0) false false)))))

(event Custom|RemovePlate
  (Variables|Default|Setactiveplates (- (Variables|Default|Getactiveplates) 1))
  (if (< (Variables|Default|Getactiveplates) (Variables|Default|GetTrigger))
    (bind _newtrack_0 (Timeline|Timeline Reverse)
      (:Update
        (Transformation|SetRelativeRotation (Variables|Debug|GetStaticMeshComponent) (Math|Rotator|Lerp(Rotator) "90.000000,0.000000,0.000000" "90.000000,90.000000,0.000000" _newtrack_0) false false)))))

(fn ConstructionScript)