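; A level pressure plate that reacts to BP_L3_PickupCube actors entering its box and reports to a linked door.
; An overlap count ensures the door gains a plate on the first cube and loses it on the last.
; If that first cube is tagged Pickup, its mesh enables custom depth and TargetActor eases to an offset from the plate's location.
; Leaving reverts neither the custom depth nor the move.
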(event OnComponentEndOverlap(Box)
  (params (OverlappedComponent :type Primitive%20Component%20Object%20Reference) (OtherActor :type Actor%20Object%20Reference) (OtherComp :type Primitive%20Component%20Object%20Reference) (OtherBodyIndex :type Integer))
  (Utilities|Casting|CastToBP_L3_PickupCube OtherActor)
  (Variables|Default|SetOverlappingObjects (- (Variables|Default|GetOverlappingObjects) 1))
  (if (== (Variables|Default|GetOverlappingObjects) 0)
    (Default|RemovePlate (Variables|Default|GetLinkedDoor))))

(event OnComponentBeginOverlap(Box)
  (params (OverlappedComponent :type Primitive%20Component%20Object%20Reference) (OtherActor :type Actor%20Object%20Reference) (OtherComp :type Primitive%20Component%20Object%20Reference) (OtherBodyIndex :type Integer) (bFromSweep :type Boolean) (SweepResult :type Hit%20Result%20Structure%20%28by%20ref%29))
  (Utilities|Casting|CastToBP_L3_PickupCube OtherActor)
  (Variables|Default|SetOverlappingObjects (+ (Variables|Default|GetOverlappingObjects) 1))
  (if (== (Variables|Default|GetOverlappingObjects) 1)
    (Default|AddPlate (Variables|Default|GetLinkedDoor))
    (if (Actor|ActorHasTag OtherActor "Pickup")
      (Rendering|SetRenderCustomDepth (Actor|GetComponentbyClass OtherActor "/Script/Engine.StaticMeshComponent") true)
      (Components|MoveComponentTo (Variables|/Script/Engine.Actor|GetRootComponent (Variables|Default|GetTargetActor)) (Variables|Default|GetFinalLocation) (Variables|Default|GetTarget%20Relative%20Rotation) true true 1.0 false))))

(event EventBeginPlay
  (Utilities|IsValid (Variables|Default|GetTargetActor)
    (:Is%20Valid
      (Variables|Default|SetFinalLocation (+ (Transformation|GetActorLocation) (Variables|Default|GetTarget%20Relative%20Location))))))

(fn ConstructionScript)