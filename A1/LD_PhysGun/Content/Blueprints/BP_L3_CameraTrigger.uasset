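; BP_L3_CameraTrigger plays a level sequence, by its name a Level 3 camera shot, when a geometry collection breaks.
; The Chaos break event waits one second, then passes a DoOnce so the sequence starts only once.
; Player input is disabled before playback but re-enabled immediately after the play call, as the bound OnFinished event is empty.
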(event OnChaosBreakEvent(GeometryCollection)
  (params (BreakEvent :type Chaos%20Break%20Event%20Structure%20%28by%20ref%29))
  (bind _ls (Variables|Default|GetLS))
  (bind _sequenceplayer (Variables|/Script/LevelSequence.LevelSequenceActor|GetSequencePlayer _ls))
  (Utilities|FlowControl|Delay 1.0)
  (Utilities|FlowControl|DoOnce false
    (:Completed
      (Input|DisableInput (Game|Player|GetPlayerPawn 0) (Game|GetPlayerController 0))
      (Sequencer|Player|Play _sequenceplayer :!class /Script/MovieScene.MovieSceneSequencePlayer)
      (EventDispatchers|AssignOnFinished _sequenceplayer (delegate Custom|OnFinished_Event))
      (Input|EnableInput (Game|Player|GetPlayerPawn 0) (Game|GetPlayerController 0)))))

(event Custom|OnFinished_Event)

(event EventBeginPlay)

(event Collision|EventActorBeginOverlap
  (params (OtherActor :type Actor%20Object%20Reference)))

(event EventTick
  (params (DeltaSeconds :type Float%20%28single-precision%29)))

(fn ConstructionScript)